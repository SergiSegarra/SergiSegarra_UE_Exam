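; Door Blueprint that opens for a ThirdPersonCharacter who has collected exactly three pickables.
; Entering its collider with that count plays a timeline, and any such character leaving reverses it without a count check.
; Timeline updates set the actor's relative location by lerping between DoorOpen and DoorClosed.
; The lerp alpha is a constant zero as written, so updates snap the door to DoorOpen rather than animating it.
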(event `self.Collider.OnComponentBeginOverlap`
  (params (OverlappedComponent :type "PrimitiveComponent Object Reference") (OtherActor :type "Actor Object Reference") (OtherComp :type "PrimitiveComponent Object Reference") (OtherBodyIndex :type Integer) (bFromSweep :type Boolean) (SweepResult :type "HitResult Structure (by ref)"))
  (bind _asthird_person_character (cast `/Game/ThirdPersonBP/Blueprints/ThirdPersonCharacter` OtherActor))
  (if (== (`/Game/ThirdPersonBP/Blueprints/ThirdPersonCharacter.PickablesCollected` _asthird_person_character) 3)
    (`Timeline|Timeline_0` :!label _label
      (:`Update`
        (`self.K2_SetActorRelativeLocation` self (`KismetMathLibrary.VLerp` (`self.DoorOpen`) (`self.DoorClosed`)) false false)))))

(event `self.Collider.OnComponentEndOverlap`
  (params (OverlappedComponent :type "PrimitiveComponent Object Reference") (OtherActor :type "Actor Object Reference") (OtherComp :type "PrimitiveComponent Object Reference") (OtherBodyIndex :type Integer))
  (cast `/Game/ThirdPersonBP/Blueprints/ThirdPersonCharacter` OtherActor)
  (goto _label :!via `Reverse`))

(fn `UserConstructionScript`)